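; BP_Door_ForestScene is the forest demo's door, which starts the outro cutscene once the slide puzzle has been solved.
; When a character finishes moving to it, it checks the scene manager's state strings for StateCondition, which the puzzle adds.
; If present, it removes the character from its map and calls BeginOutroCutscene on BP_ForestDemoSceneManager.
; Otherwise it defers to the parent door's move-completion behavior.
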(fn ConstructionScript
  (|CallParentFunction))

(fn OnCharacterMoveCompletion
  (params (Character :type BP%20PNC%20Character%20Parent%20Object%20Reference))
  (if (Utilities|Array|ContainsItem (Default|GetStateStrings (CallFunction|GetSceneManager)) (Variables|Default|GetStateCondition))
    (CallFunction|RemoveCharacterfromMap Character)
    (bind _asbp_forest_demo_scene_manager (Utilities|Casting|CastToBP_ForestDemoSceneManager (CallFunction|GetSceneManager))
      (:then
        (Default|BeginOutroCutscene _asbp_forest_demo_scene_manager)
        (return false))
      (:CastFailed
        (return true)))
    (else
      (bind _return (|CallParentFunction Character))
      (return _return))))